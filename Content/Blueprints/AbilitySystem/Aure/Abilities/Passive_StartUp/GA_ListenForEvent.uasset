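; Gameplay ability in the passive start-up set that turns Attribute gameplay events into changes on its owner.
; On activation it waits for events under the Attribute tag, including child tags.
; Each event builds a fresh EventBasedEffectClass spec, looping over EventTags to assign zero SetByCaller magnitudes.
; It then sets the event's tag to the payload magnitude and applies the spec to itself.
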(event `self.K2_ActivateAbility`
  (bind (_asynctaskproxy _payload) (`AbilityTask_WaitGameplayEvent.WaitGameplayEvent` (struct :`TagName` "Attribute") null false false)
    (:`EventReceived`
      (bind _gespec (`self.MaKe GESpec`))
      (bind (_eventtag _instigator _target _optionalobject _optionalobject2 _contexthandle _instigatortags _targettags _eventmagnitude) (break `GameplayEventData` _payload))
      (bind _returnvalue (`AbilitySystemBlueprintLibrary.AssignTagSetByCallerMagnitude` _gespec _eventtag _eventmagnitude))
      (`AbilitySystemComponent.BP_ApplyGameplayEffectSpecToSelf` (`self.GetAbilitySystemComponentFromActorInfo`) _returnvalue))))

(fn `MaKe GESpec`
  (returns (GESpec :type "GameplayEffectSpecHandle Structure"))
  (bind _returnvalue (`self.GetAbilitySystemComponentFromActorInfo`))
  (set `self.GESpec` (`AbilitySystemComponent.MakeOutgoingSpec` _returnvalue (`self.EventBasedEffectClass`) 1.0 (`AbilitySystemComponent.MakeEffectContext` _returnvalue)))
  (for _ (`self.Event Tags`)
    (`AbilitySystemBlueprintLibrary.AssignTagSetByCallerMagnitude` (`self.GESpec`)))
  (return (`self.GESpec`)))