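; BP_Pillar is a dungeon pillar Blueprint that continuously animates the intensity of its point light.
; On BeginPlay it randomly picks one of two timelines, each scaling the light by a base brightness variable through its float track.
; When a timeline finishes, it triggers another random pick, so the light varies in an endless loop without using Tick.
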(event `self.ReceiveBeginPlay`
  (`self.ChooseTimeline`))

(event `StartTimeline_1`
  (bind (_direction `_新建轨道_0`) (`Timeline|时间轴`)
    (:`Update`
      (`LightComponent.SetIntensity` (`self.PointLight`) (* `_新建轨道_0` (`self.初始亮度`))))
    (:`Finished`
      (`self.ChooseTimeline`))))

(event `StartTimeline_2`
  (bind (_direction `_新建轨道_0`) (`Timeline|时间轴_0`)
    (:`Update`
      (`LightComponent.SetIntensity` (`self.PointLight`) (* `_新建轨道_0` (`self.初始亮度`))))
    (:`Finished`
      (`self.ChooseTimeline`))))

(event `ChooseTimeline`
  (switch `int` (`KismetMathLibrary.RandomIntegerInRange` 0 1)
    (:`Default`
      (`self.StartTimeline_1` :!label _label))
    (:`0`
      (goto _label))
    (:`1`
      (`self.StartTimeline_2`))))

(fn `UserConstructionScript`)