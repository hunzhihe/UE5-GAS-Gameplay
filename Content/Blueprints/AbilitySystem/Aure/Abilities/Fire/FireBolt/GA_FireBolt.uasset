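; GA_FireBolt is a gameplay ability that casts fire bolt projectiles at the target under the mouse.
; On activation it commits, takes the hit location and actor from a mouse target data task, and turns the avatar toward that point through CombatInterface.
; It plays the cast montage, waits for its gameplay event, then spawns homing projectiles from the weapon socket.
; The ability ends shortly after spawning or when the montage finishes or aborts.
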(event `self.K2_ActivateAbility`
  (`self.K2_CommitAbility`)
  (bind (_asynctaskproxy _datahandle) (`TagetUnderMouse_AbilityTask.CreateTagetDataUnderMouse_AbilityTask`)
    (:`ValidData`
      (bind (_bblockinghit _binitialoverlap _time _distance _location _impactpoint _normal _impactnormal _physmat _hitactor) (`GameplayStatics.BreakHitResult` (`AbilitySystemBlueprintLibrary.GetHitResultFromTargetData` _datahandle)))
      (bind _output_get (set `self.Location` _location))
      (set `self.HomingTarget` _hitactor)
      (bind _ascombat_interface (cast `CombatInterface` (`self.GetAvatarActorFromActorInfo`)))
      (`CombatInterface.FaceingTarget` _ascombat_interface _output_get)
      (`AbilityTask_PlayMontageAndWait.CreatePlayMontageAndWaitProxy` "None" "/Game/Assets/Characters/Aura/Animations/Abilities/AM_Cast_FireBolt_Montage.AM_Cast_FireBolt_Montage"
        (:`then`
          (`AbilityTask_WaitGameplayEvent.WaitGameplayEvent` (struct :`TagName` "Event.Montage.FireBolt") null
            (:`EventReceived`
              (`self.SpawnProjectliles` (`self.Location`) (`BlueprintGameplayTagLibrary.MakeLiteralGameplayTag` (struct :`TagName` "CombatSocket.Weapon")) "None" false 0.0 (`self.HomingTarget`))
              (`KismetSystemLibrary.Delay` 0.5)
              (`self.K2_EndAbility`))))
        (:`OnCompleted`
          (`self.K2_EndAbility` :!label _label))
        (:`OnBlendOut`
          (goto _label))
        (:`OnInterrupted`
          (goto _label))
        (:`OnCancelled`
          (goto _label))))))