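; Enemy melee attack gameplay ability that turns the avatar toward its combat target and plays a random tagged attack montage.
; On the montage's gameplay event, it runs a radius overlap at the tagged combat socket, applying damage and blood effects to hostile live actors.
; Any hit fires a MeleeImpact gameplay cue tagged with the montage tag.
; A debug sphere shows the hit area, and the ability ends after the event or montage end.
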(event `self.K2_ActivateAbility`
  (bind _returnvalue (`self.GetAvatarActorFromActorInfo`))
  (bind _returnvalue_2 (`self.GetAvatarActorFromActorInfo`))
  (set `self.HasHitTarget` false)
  (bind _returnvalue_3 (message `EnemyInterface.GetCombatTarget` _returnvalue_2))
  (bind _ascombat_interface (cast `CombatInterface` _returnvalue_2))
  (`CombatInterface.FaceingTarget` _ascombat_interface (`Actor.K2_GetActorLocation` _returnvalue_3))
  (bind _returnvalue_4 (message `CombatInterface.GetAttackMontages` _returnvalue_2))
  (bind _output_get (set `self.TaggedMontage` (`self.GetRandomTaggedMontageFromArray` _returnvalue_4)))
  (bind (_montage _montagetag _sockettag) (break `TaggedMontage` _output_get))
  (`AbilityTask_PlayMontageAndWait.CreatePlayMontageAndWaitProxy` "None" _montage 1.0 "None" false
    (:`then`
      (`AbilityTask_WaitGameplayEvent.WaitGameplayEvent` _montagetag null
        (:`EventReceived`
          (bind _returnvalue_5 (message `CombatInterface.GetCombatSocketLocation` _returnvalue _sockettag))
          (bind _output_get_2 (set `self.Socket Location` _returnvalue_5))
          (bind _outoverlappingactors (`AureAbilitySysTEM_BFL.GetLivePlayerWithRadius` _returnvalue (`|MakeArray` _returnvalue) 50.0 _output_get_2))
          (`KismetSystemLibrary.DrawDebugSphere` (`self.Socket Location`) 50.0 12 (struct :`R` 1.0 :`G` 0.151042 :`B` 0.151042 :`A` 1.0) 5.0)
          (for _array_element _outoverlappingactors
            (if (`AureAbilitySysTEM_BFL.IsEnemy` (`self.GetAvatarActorFromActorInfo`) _array_element)
              (`self.ExecuteDamageEffect` _array_element)
              (set `self.HasHitTarget` true)
              (message `CombatInterface.GetBloodEffect` _array_element)))
          (if (`self.HasHitTarget`)
            (bind _returnvalue_6 (message `EnemyInterface.GetCombatTarget` (`self.GetAvatarActorFromActorInfo`)))
            (`self.K2_ExecuteGameplayCueWithParams` (struct :`TagName` "GameplayCue.MeleeImpact") (`AbilitySystemBlueprintLibrary.MakeGameplayCueParameters` 0.0 0.0 (struct) (struct) (struct) (`BlueprintGameplayTagLibrary.MakeGameplayTagContainerFromTag` (`.MontageTag` (break `TaggedMontage` (`self.TaggedMontage`)))) (struct) (`self.Socket Location`) (0.0 0.0 0.0) null (`self.GetAvatarActorFromActorInfo`) _returnvalue_6)))
          (`self.K2_EndAbility`))))
    (:`OnCompleted`
      (`self.K2_EndAbility` :!label _label))
    (:`OnInterrupted`
      (goto _label))
    (:`OnCancelled`
      (goto _label))))