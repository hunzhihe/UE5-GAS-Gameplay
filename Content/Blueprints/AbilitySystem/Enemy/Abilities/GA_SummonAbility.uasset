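; Enemy gameplay ability that summons random minions around the caster using the Shaman summon montage.
; It shuffles computed spawn locations, plays ground Niagara effects at each, then waits for the weapon socket gameplay event.
; A delayed loop spawns AI-controlled minions one by one, facing away from the caster.
; The caster's minion count rises per spawn and falls on destruction; montage completion, blend-out or cancellation ends the ability.
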(event `self.K2_ActivateAbility`
  (bind _output (`|GetArrayItem` (`self.SpawnLocation`) (`self.SpawnLocationIndex`)))
  (bind _returnvalue (`self.GetSpawnLocations`))
  (bind _output_get (set `self.SpawnLocation` _returnvalue))
  (`KismetArrayLibrary.Array_Shuffle` _output_get)
  (`|ExecutionSequence`
    (:`then_0`
      (for _array_element (`self.SpawnLocation`)
        (`NiagaraFunctionLibrary.SpawnSystemAtLocation` "/Game/Assets/Effects/Combat/NS_GroundSummon.NS_GroundSummon" _array_element (struct) (1.0 1.0 1.0) true true "AutoRelease")))
    (:`then_1`
      (`AbilityTask_PlayMontageAndWait.CreatePlayMontageAndWaitProxy` "None" "/Game/Assets/Enemies/Shaman/Animations/AM_Shaman_Summon.AM_Shaman_Summon"
        (:`then`
          (`AbilityTask_WaitGameplayEvent.WaitGameplayEvent` (struct :`TagName` "CombatSocket.Weapon") null
            (:`EventReceived`
              (set `self.SpawnLocationIndex` 0)
              (if (< (`self.SpawnLocationIndex`) (`KismetArrayLibrary.Array_Length` (`self.SpawnLocation`))) :!label _label
                (bind _returnvalue_2 (`|SpawnActorFromClass` (`self.GetRandomMinionClass`) (`KismetMathLibrary.MakeTransform` (+ _output (0.0 0.0 70.0)) (`KismetMathLibrary.FindLookAtRotation` (`Actor.K2_GetActorLocation` (`self.GetAvatarActorFromActorInfo`)) _output)) "AdjustIfPossibleButAlwaysSpawn" "MultiplyWithRoot" null null))
                (`Pawn.SpawnDefaultController` _returnvalue_2)
                (add `Actor.OnDestroyed` _returnvalue_2 (delegate `OnDestroyed_事件`))
                (message `CombatInterface.IncrementMinionsCount` (`self.GetAvatarActorFromActorInfo`) 1)
                (`/Engine/EditorBlueprintResources/StandardMacros.IncrementInt` (`self.SpawnLocationIndex`)
                  (:`  `
                    (`KismetSystemLibrary.Delay` 0.2)
                    (goto _label)))))))
        (:`OnCompleted`
          (`self.K2_EndAbility` :!label _label_2))
        (:`OnBlendOut`
          (goto _label_2))
        (:`OnCancelled`
          (goto _label_2))))))

(event `OnDestroyed_事件`
  (params (DestroyedActor :type "Actor Object Reference"))
  ; 监听召唤物死亡时，减少召唤物数量
  (message `CombatInterface.IncrementMinionsCount` (`self.GetAvatarActorFromActorInfo`) -1))